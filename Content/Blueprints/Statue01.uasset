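; Statue01 is an actor that passes an emitting state to another statue it faces, forming a chain of beams.
; On Tick, after a short Delay, an emitting statue runs a forward Visibility line trace with one-frame debug drawing.
; When the trace hits another Statue01, it sets that statue's Emitindo flag to true, and nothing in this graph ever clears it.
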(event EventTick
  (params (DeltaSeconds :type Float%20%28single-precision%29))
  (bind _returnvalue (Transformation|GetActorLocation))
  (Utilities|FlowControl|Delay 0.01)
  (if (Variables|Default|GetEmitindo?)
    (bind (_outhit _returnvalue_2) (Collision|LineTraceByChannel _returnvalue (+ _returnvalue (* (Transformation|GetActorForwardVector) 1000)) "TraceTypeQuery1" false 0 "ForOneFrame"))
    (if _returnvalue_2
      (bind _asstatue_01 (Utilities|Casting|CastToStatue01 (.HitActor (Collision|BreakHitResult _outhit))))
      (Variables|Statue01_C|SetEmitindo? _asstatue_01 true))))

(fn ConstructionScript)