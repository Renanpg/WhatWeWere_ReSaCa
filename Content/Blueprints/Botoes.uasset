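; A puzzle button that responds to a PickUpable2 box with a matching ID and drives two linked doors.
; When the correct box enters its trigger, a flag guards a single increment of both doors' open counts; when it leaves, both counts decrease.
; A wrong box entering clears that flag without decrementing the doors.
; Pressed and released timelines for moving the button vertically exist but are never run.
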(event OnComponentBeginOverlap(Box)
  (params (OverlappedComponent :type Primitive%20Component%20Object%20Reference) (OtherActor :type Actor%20Object%20Reference) (OtherComp :type Primitive%20Component%20Object%20Reference) (OtherBodyIndex :type Integer) (bFromSweep :type Boolean) (SweepResult :type Hit%20Result%20Structure%20%28by%20ref%29))
  (bind _aspick_upable_2 (Utilities|Casting|CastToPickUpable2 OtherActor))
  (if (== (Variables|/Game/Blueprints/PickUpable2.PickUpable2_C|GetID%20da%20caixa _aspick_upable_2) (Variables|Default|GetID%20correto))
    (if (not (Variables|Default|GetAbriu?))
      (Variables|Default|SetAbriu? true)
      (Default|SomaAbertos (Variables|Default|GetDoors))
      (Default|SomaAbertos (Variables|Default|GetDoors2)))
    (else
      (Variables|Default|SetAbriu? false))))

(event OnComponentEndOverlap(Box)
  (params (OverlappedComponent :type Primitive%20Component%20Object%20Reference) (OtherActor :type Actor%20Object%20Reference) (OtherComp :type Primitive%20Component%20Object%20Reference) (OtherBodyIndex :type Integer))
  (bind _aspick_upable_2 (Utilities|Casting|CastToPickUpable2 OtherActor))
  (if (== (Variables|/Game/Blueprints/PickUpable2.PickUpable2_C|GetID%20da%20caixa _aspick_upable_2) (Variables|Default|GetID%20correto))
    (Variables|Default|SetAbriu? false)
    (Default|ReduzAbertos (Variables|Default|GetDoors))
    (Default|ReduzAbertos (Variables|Default|GetDoors2))))

(fn ConstructionScript)