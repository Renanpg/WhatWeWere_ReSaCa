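; Door actor that slides open once a counter, Abertos, reaches at least three.
; SomaAbertos increments the counter and ReduzAbertos decrements it, both printing the value; decrementing never closes the door.
; At the threshold, PortaDireita selects one of two timelines, which drives the actor's world Y as track value times PositionA or PositionB, keeping X and Z.
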(event Custom|SomaAbertos
  (bind _returnvalue (Transformation|GetActorLocation))
  (bind _abertos (Variables|Default|GetAbertos))
  (Math|Integer|IncrementInt _abertos
    (:%20%20
      (Development|PrintString (Utilities|String|ToString(Integer) _abertos))
      (if (>= _abertos 3)
        (if (Variables|Default|GetPortaDireita?)
          (bind _newtrack_0 (Timeline|AnimAberturaA Play)
            (:Update
              (Transformation|SetActorLocation (Math|Vector|MakeVector (.x _returnvalue) (* _newtrack_0 (Variables|Default|GetPositionA)) (.z _returnvalue)) false false)))
          (else
            (bind _newtrack_0_2 (Timeline|AnimAberturaB Play)
              (:Update
                (Transformation|SetActorLocation (Math|Vector|MakeVector (.x _returnvalue) (* _newtrack_0_2 (Variables|Default|GetPositionB)) (.z _returnvalue)) false false)))))))))

(event Custom|ReduzAbertos
  (bind _abertos (Variables|Default|GetAbertos))
  (Math|Integer|DecrementInt _abertos
    (:%20%20
      (Development|PrintString (Utilities|String|ToString(Integer) _abertos)))))

(event Collision|EventActorBeginOverlap
  (params (OtherActor :type Actor%20Object%20Reference)))

(event EventTick
  (params (DeltaSeconds :type Float%20%28single-precision%29)))

(fn ConstructionScript)